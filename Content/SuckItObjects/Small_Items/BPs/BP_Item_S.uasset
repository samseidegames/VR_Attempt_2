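; BP_Item_S is a small suckable item whose construction script sets a mesh and mass from the chosen item type (Bench or Cutting Table).
; BeginPlay caches the BP_Tank and VRPawn, and PullTowardsTank moves the item toward the tank at a frame-scaled speed.
; Tick and overlap events are empty.
; The pull trigger and the absorb logic that destroys the item and adds its mass to the pawn's total are disconnected.
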(event `self.ReceiveBeginPlay`
  ;[0.03434 0.03434 0.03434] Gets our Tank Instance
  (bind _outactors (`GameplayStatics.GetAllActorsOfClass` "/Game/SuckItObjects/BP_Tank.BP_Tank_C"))
  (for _array_element _outactors
    (if (`KismetSystemLibrary.IsValid` _array_element)
      (set `self.TankReference` _array_element)
      (bind _outactors_2 (`GameplayStatics.GetAllActorsOfClass` "/Game/VRTemplate/Blueprints/VRPawn.VRPawn_C"))
      (for _array_element_2 _outactors_2
        (set `self.VRPawnReference` _array_element_2)))))

(event `self.ReceiveTick`
  (params (DeltaSeconds :type "Float (single-precision)")))

(event `self.SuckCollission.OnComponentBeginOverlap`
  (params (OverlappedComponent :type "PrimitiveComponent Object Reference") (OtherActor :type "Actor Object Reference") (OtherComp :type "PrimitiveComponent Object Reference") (OtherBodyIndex :type Integer) (bFromSweep :type Boolean) (SweepResult :type "HitResult Structure (by ref)")))

(event `self.SuckCollission.OnComponentEndOverlap`
  (params (OverlappedComponent :type "PrimitiveComponent Object Reference") (OtherActor :type "Actor Object Reference") (OtherComp :type "PrimitiveComponent Object Reference") (OtherBodyIndex :type Integer)))

(event `PullTowardsTank`
  (`self.K2_AddActorLocalOffset` (* (`KismetMathLibrary.Normal` (- (`self.K2_GetActorLocation` (`self.TankReference`)) (`self.K2_GetActorLocation`))) (`GameplayStatics.GetWorldDeltaSeconds`) (`self.Speed`))))

(event `self.ItemCollission.OnComponentBeginOverlap`
  (params (OverlappedComponent :type "PrimitiveComponent Object Reference") (OtherActor :type "Actor Object Reference") (OtherComp :type "PrimitiveComponent Object Reference") (OtherBodyIndex :type Integer) (bFromSweep :type Boolean) (SweepResult :type "HitResult Structure (by ref)")))

(fn `UserConstructionScript`
  (bind _item (`self.Item`))
  (switch `/Game/SuckItObjects/Small_Items/BPs/SItemMeshOptions` (`self.ItemMesh`)
    (:`NewEnumerator0`
      (`StaticMeshComponent.SetStaticMesh` _item "/Game/SuckItObjects/Small_Items/Bench.Bench")
      (set `self.ItemMesh` "NewEnumerator0")
      (set `self.ItemMass` 12.0))
    (:`NewEnumerator3`
      (`StaticMeshComponent.SetStaticMesh` _item "/Game/SuckItObjects/Small_Items/CuttingTable.CuttingTable")
      (set `self.ItemMesh` "NewEnumerator3")
      (set `self.ItemMass` 6.0))))