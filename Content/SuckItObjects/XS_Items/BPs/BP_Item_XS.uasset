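; Extra-small item that the tank sucks up to gain weight, with mesh and mass chosen from a food-and-bottle variant in the construction script.
; After the tank overlaps SuckCollission, Tick pulls the item toward it; the tank-weight check is left unconnected.
; Touching ItemCollission destroys the item, adds its mass to the VRPawn's total and rescales tank and pawn once that passes the small-size threshold.
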(event `self.ReceiveBeginPlay`
  ;[1 1 1] Gets our Tank Instance
  (bind _outactors (`GameplayStatics.GetAllActorsOfClass` "/Game/SuckItObjects/BP_Tank.BP_Tank_C"))
  (for _array_element _outactors
    (if (`KismetSystemLibrary.IsValid` _array_element)
      (set `self.TankReference` _array_element)
      (bind _outactors_2 (`GameplayStatics.GetAllActorsOfClass` "/Game/VRTemplate/Blueprints/VRPawn.VRPawn_C"))
      (for _array_element_2 _outactors_2
        (set `self.VRPawnReference` _array_element_2)))))

(event `self.ReceiveTick`
  (params (DeltaSeconds :type "Float (single-precision)"))
  ;[1 1 1] If tank weight is bigger than x-small size pull the object towards the tank
  (bind _tanksizemax (`/Game/SuckItObjects/General_BPs/TankSizeGlobals.Get X-Small Tank Size`))
  (if true
    (`self.Other Actor`
      (:`then`
        (`self.PullTowardsTank`))
      (:`else`))))

(event `self.SuckCollission.OnComponentBeginOverlap`
  (params (OverlappedComponent :type "PrimitiveComponent Object Reference") (OtherActor :type "Actor Object Reference") (OtherComp :type "PrimitiveComponent Object Reference") (OtherBodyIndex :type Integer) (bFromSweep :type Boolean) (SweepResult :type "HitResult Structure (by ref)"))
  (if (== OtherActor (`self.TankReference`))
    (set `self.Other Actor` OtherActor)))

(event `PullTowardsTank`
  ;[1 1 1] Pull Item Towards Tank
  (`self.K2_AddActorLocalOffset` (* (`KismetMathLibrary.Normal` (- (`self.K2_GetActorLocation` (`self.TankReference`)) (`self.K2_GetActorLocation`))) (`GameplayStatics.GetWorldDeltaSeconds`) (`self.Speed`))))

(event `self.ItemCollission.OnComponentBeginOverlap`
  (params (OverlappedComponent :type "PrimitiveComponent Object Reference") (OtherActor :type "Actor Object Reference") (OtherComp :type "PrimitiveComponent Object Reference") (OtherBodyIndex :type Integer) (bFromSweep :type Boolean) (SweepResult :type "HitResult Structure (by ref)"))
  (bind _itemcollission (`self.ItemCollission`))
  (bind _suckcollission (`self.SuckCollission`))
  (bind _vrpawnreference (`self.VRPawnReference`))
  ;[1 1 1] when the tank touches the ItemCollission destroy our item and increase tank size
  (if (== OtherActor (`self.TankReference`))
    (`PrimitiveComponent.SetCollisionEnabled` (`self.Item`) "NoCollision")
    (`/Engine/EditorBlueprintResources/StandardMacros.IsValid` _itemcollission
      (:`Is Valid`
        (`PrimitiveComponent.SetCollisionEnabled` _itemcollission "NoCollision"))
      (:`Is Not Valid`
        _))
    (`/Engine/EditorBlueprintResources/StandardMacros.IsValid` _suckcollission
      (:`Is Valid`
        (`PrimitiveComponent.SetCollisionEnabled` _suckcollission "NoCollision"))
      (:`Is Not Valid`
        _))
    (`self.K2_DestroyActor`)
    (`/Game/VRTemplate/Blueprints/VRPawn.UpdateTotalWeight` _vrpawnreference (`self.ItemMass`))
    (bind _tanksizemax (`/Game/SuckItObjects/General_BPs/TankSizeGlobals.Get Small Tank Size`))
    (if (> (`/Game/VRTemplate/Blueprints/VRPawn.TankTotalWeight` _vrpawnreference) _tanksizemax)
      (`SceneComponent.SetWorldScale3D` (`Actor.RootComponent` (`self.TankReference`)) (0.2 0.2 0.2))
      (`SceneComponent.SetWorldScale3D` (`Actor.RootComponent` (`self.VRPawnReference`)) (0.2 0.2 0.2)))))

(fn `UserConstructionScript`
  (bind _item (`self.Item`))
  (switch `/Game/SuckItObjects/XS_Items/BPs/XSItemMeshOptions` (`self.ItemMesh`)
    (:`NewEnumerator3`
      (`StaticMeshComponent.SetStaticMesh` _item "/Game/SuckItObjects/XS_Items/Avocado.Avocado")
      (set `self.ItemMesh` "NewEnumerator3")
      (set `self.ItemMass` 0.154))
    (:`NewEnumerator4`
      (`StaticMeshComponent.SetStaticMesh` _item "/Game/SuckItObjects/XS_Items/Bottle.Bottle")
      (set `self.ItemMesh` "NewEnumerator4")
      (set `self.ItemMass` 0.71))
    (:`NewEnumerator1`
      (`StaticMeshComponent.SetStaticMesh` _item "/Game/SuckItObjects/XS_Items/Ramen.Ramen")
      (set `self.ItemMesh` "NewEnumerator1")
      (set `self.ItemMass` 0.3))
    (:`NewEnumerator2`
      (`StaticMeshComponent.SetStaticMesh` _item "/Game/SuckItObjects/XS_Items/SeaUrchinRoll.SeaUrchinRoll")
      (set `self.ItemMesh` "NewEnumerator2")
      (set `self.ItemMass` 0.4))
    (:`NewEnumerator0`
      (`StaticMeshComponent.SetStaticMesh` _item "/Game/SuckItObjects/XS_Items/Udon.Udon")
      (set `self.ItemMesh` "NewEnumerator0")
      (set `self.ItemMass` 0.255))))