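; Extra-small suckable pickup that is pulled toward the player and adds its mass to the tank's weight when collected.
; BeginPlay picks a random DT_SuckItItems row for mesh and data, then finds BP_Tank.
; SuckCollission overlap stores the player as target, and Tick moves the item toward it.
; ItemCollission overlap updates TankInfo weight and the tank's display, destroys the item, and rescales the tank above a weight threshold.
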(event `self.ReceiveBeginPlay`
  ;[1 1 1] BeginPlay
  (bind _outrownames (`DataTableFunctionLibrary.GetDataTableRowNames` "/Game/SuckItObjects/Data_Tables/DT_SuckItItems.DT_SuckItItems"))
  (bind _returnvalue (`|GetDataTableRow` "/Game/SuckItObjects/Data_Tables/DT_SuckItItems.DT_SuckItItems" (`|GetArrayItem` _outrownames (`KismetMathLibrary.RandomIntegerInRange` 0 (- (`KismetArrayLibrary.Array_Length` _outrownames) 1))))
    (:`then`
      (bind _output_get (set `self.BaseInfo` _returnvalue))
      (`StaticMeshComponent.SetStaticMesh` (`self.Item`) (`.Mesh_12_8E714C364DD81D518DA64684CA241D6F` (break `/Game/SuckItObjects/Structures/Struct_suckItItem` _output_get)))
      ;[1 1 1] Gets our Tank Instance
      (bind _outactors (`GameplayStatics.GetAllActorsOfClass` "/Game/SuckItObjects/BP_Tank.BP_Tank_C"))
      (for _array_element _outactors
        (if (`KismetSystemLibrary.IsValid` _array_element)
          (set `self.TankReference` _array_element))))))

(event `self.ReceiveTick`
  (params (DeltaSeconds :type "Float (single-precision)"))
  ;[1 1 1] If tank weight is bigger than x-small size pull the object towards the tank
  (`self.Other Actor`
    (:`then`
      (`self.PullTowardsTank`)
      (`KismetSystemLibrary.PrintString` "Pull Towards Tank Activated"))
    (:`else`)))

(event `PullTowardsTank`
  ;[1 1 1] Pull Item Towards Tank
  (`KismetSystemLibrary.PrintString` "Pulling in object")
  (bind _output_get (set `self.PullSpeed` 30.0))
  (`self.K2_AddActorLocalOffset` (* (`KismetMathLibrary.Normal` (- (`self.K2_GetActorLocation` (`self.Other Actor`)) (`self.K2_GetActorLocation`))) (`GameplayStatics.GetWorldDeltaSeconds`) _output_get)))

(event `self.ItemCollission.OnComponentBeginOverlap`
  (params (OverlappedComponent :type "PrimitiveComponent Object Reference") (OtherActor :type "Actor Object Reference") (OtherComp :type "PrimitiveComponent Object Reference") (OtherBodyIndex :type Integer) (bFromSweep :type Boolean) (SweepResult :type "HitResult Structure (by ref)"))
  (bind _itemcollission (`self.ItemCollission`))
  (bind _suckcollission (`self.SuckCollission`))
  (bind (_tankinfo_rotation _tankinfo_speed_r _tankinfo_speed_l _tankinfo_speed_total _tankinfo_scale _tankinfo_weight) (break `/Game/SuckItObjects/Structures/Struct_Tank` (`self.TankInfo`)))
  (bind (_baseinfo_speed _baseinfo_maxspeed _baseinfo_scale _baseinfo_mesh _baseinfo_itemmass) (break `/Game/SuckItObjects/Structures/Struct_suckItItem` (`self.BaseInfo`)))
  ;[1 1 1] On Overlap ItemCollission
  (if (== null (`GameplayStatics.GetPlayerCharacter` 0))
    (set `self.Other Actor` null)
    (`KismetSystemLibrary.PrintString` "ItemCollission")
    (`PrimitiveComponent.SetCollisionEnabled` (`self.Item`) "NoCollision")
    (`/Engine/EditorBlueprintResources/StandardMacros.IsValid` _itemcollission
      (:`Is Valid`
        (`PrimitiveComponent.SetCollisionEnabled` _itemcollission "NoCollision"))
      (:`Is Not Valid`
        _))
    (`/Engine/EditorBlueprintResources/StandardMacros.IsValid` _suckcollission
      (:`Is Valid`
        (`PrimitiveComponent.SetCollisionEnabled` _suckcollission "NoCollision")
        (bind _structout (setmembers `/Game/SuckItObjects/Structures/Struct_Tank` :`StructRef` (`self.TankInfo`) :`Weight` (+ _tankinfo_weight _baseinfo_itemmass)))
        (bind _output_get (set `self.TankInfo` _structout))
        (`TextRenderComponent.K2_SetText` (`/Game/SuckItObjects/BP_Tank.CurrentWeightDisplay` (`self.TankReference`)) (`KismetTextLibrary.Conv_DoubleToText` (`.Weight_12_E4551C944BF62DBF6C1C3A9AA8E3A29C` (break `/Game/SuckItObjects/Structures/Struct_Tank` _output_get)) "HalfToEven"))
        (`self.K2_DestroyActor`)
        (if (> (`.Weight_12_E4551C944BF62DBF6C1C3A9AA8E3A29C` (break `/Game/SuckItObjects/Structures/Struct_Tank` _output_get)) 0.25)
          (`/Game/SuckItObjects/BP_Tank.setTankScale` (`self.TankReference`)))))))

(event `self.SuckCollission.OnComponentBeginOverlap`
  (params (OverlappedComponent :type "PrimitiveComponent Object Reference") (OtherActor :type "Actor Object Reference") (OtherComp :type "PrimitiveComponent Object Reference") (OtherBodyIndex :type Integer) (bFromSweep :type Boolean) (SweepResult :type "HitResult Structure (by ref)"))
  ;[1 1 1] On Overlap SuckCollission
  (`KismetSystemLibrary.PrintString` (`KismetSystemLibrary.GetDisplayName` OtherActor))
  (if (== OtherActor (`GameplayStatics.GetPlayerPawn` 0))
    (`KismetSystemLibrary.PrintString` "SuckCollission")
    (set `self.Other Actor` OtherActor)))

(fn `UserConstructionScript`
  (bind _item (`self.Item`))
  (switch `/Game/SuckItObjects/XS_Items/BPs/XSItemMeshOptions` "NewEnumerator0"
    (:`NewEnumerator3`
      (`StaticMeshComponent.SetStaticMesh` _item "/Game/SuckItObjects/XS_Items/Avocado.Avocado"))
    (:`NewEnumerator4`
      (`StaticMeshComponent.SetStaticMesh` _item "/Game/SuckItObjects/XS_Items/Bottle.Bottle"))
    (:`NewEnumerator1`
      (`StaticMeshComponent.SetStaticMesh` _item "/Game/SuckItObjects/XS_Items/Ramen.Ramen"))
    (:`NewEnumerator2`
      (`StaticMeshComponent.SetStaticMesh` _item "/Game/SuckItObjects/XS_Items/SeaUrchinRoll.SeaUrchinRoll"))
    (:`NewEnumerator0`
      (`StaticMeshComponent.SetStaticMesh` _item "/Game/SuckItObjects/XS_Items/Udon.Udon"))))