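; BP_SuckItItem is a collectible item that BP_Tank sucks in, growing heavier and larger with each one.
; The construction script loads its mesh and stats from DT_SuckItItems using the ItemMeshSelection enum.
; Each Tick tests its suck sphere against the tank's, moving it toward the destroy point at a speed from suck level and tank scale.
; On reaching that point while pulling, it updates tank weight, display, scale and camera arm, then destroys itself.
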(event `self.ReceiveBeginPlay`
  ;[1 1 1] Event Begin Play
  (bind _outactors (`GameplayStatics.GetAllActorsOfClass` "/Game/SuckItObjects/BP_Tank.BP_Tank_C"))
  (for _array_element _outactors
    (if (`KismetSystemLibrary.IsValid` _array_element)
      (set `self.TankReference` _array_element))))

(event `self.ReceiveTick`
  (params (DeltaSeconds :type "Float (single-precision)"))
  (bind _item (`self.Item`))
  (bind (_origin _boxextent _sphereradius) (`KismetSystemLibrary.GetComponentBounds` (`self.SuckCollission`)))
  ;[1 1 1] Event Tick - pull towards tank when overlapping
  (bind (_hitlocation _hitnormal _bonename _outhit _returnvalue) (`PrimitiveComponent.K2_SphereOverlapComponent` (`/Game/SuckItObjects/BP_Tank.TankSuckCollision` (`self.TankReference`)) _origin _sphereradius true false false))
  (if _returnvalue
    (`self.PullTowardsTank`)
    (if (`KismetSystemLibrary.IsValid` _item)
      (`PrimitiveComponent.SetEnableGravity` _item true)
      (set `self.Pulling?` false))))

(event `PullTowardsTank`
  (bind (_tankinfo_rotation _tankinfo_speed_r _tankinfo_speed_l _tankinfo_speed_total _tankinfo_scale _tankinfo_weight _tankinfo_fuellevel _tankinfo_sucklevel) (break `/Game/SuckItObjects/Structures/Struct_Tank` (`/Game/SuckItObjects/BP_Tank.TankInfo` (`self.TankReference`))))
  (bind _returnvalue_x (`KismetMathLibrary.BreakVector` (`SceneComponent.K2_GetComponentScale` (`/Game/SuckItObjects/BP_Tank.Tank` (`self.TankReference`)))))
  ;[1 1 1] Pull Item Towards Tank if the tank is touching the items suckCollission
  (`PrimitiveComponent.SetEnableGravity` (`self.Item`) false)
  (set `self.Pulling?` true)
  (bind _output_get (set `self.PullSpeed` (* _tankinfo_sucklevel _returnvalue_x)))
  (`self.K2_AddActorWorldOffset` (* (`KismetMathLibrary.Normal` (- (`SceneComponent.K2_GetComponentLocation` (`/Game/SuckItObjects/BP_Tank.ItemCollisionDestroyPoint` (`self.TankReference`))) (`SceneComponent.K2_GetComponentLocation` (`self.ItemCollission`)))) (`GameplayStatics.GetWorldDeltaSeconds`) _output_get)))

(event `self.ItemCollission.OnComponentBeginOverlap`
  (params (OverlappedComponent :type "PrimitiveComponent Object Reference") (OtherActor :type "Actor Object Reference") (OtherComp :type "PrimitiveComponent Object Reference") (OtherBodyIndex :type Integer) (bFromSweep :type Boolean) (SweepResult :type "HitResult Structure (by ref)"))
  (bind _tankreference (`self.TankReference`))
  (bind (_tankinfo_rotation _tankinfo_speed_r _tankinfo_speed_l _tankinfo_speed_total _tankinfo_scale _tankinfo_weight) (break `/Game/SuckItObjects/Structures/Struct_Tank` (`/Game/SuckItObjects/BP_Tank.TankInfo` _tankreference)))
  (bind _returnvalue (+ 1.0 (/ _tankinfo_weight 100.0)))
  ;[1 1 1] On Overlap ItemCollission time to destroy our item
  (`KismetSystemLibrary.PrintString` "Hello")
  (if (and (`self.Pulling?`) (`PrimitiveComponent.IsOverlappingComponent` (`self.ItemCollission`) (`/Game/SuckItObjects/BP_Tank.ItemCollisionDestroyPoint` (`self.TankReference`))))
    (`/Game/SuckItObjects/BP_Tank.updateWeight` _tankreference (`.ItemMass_15_C85A45C54AA119EA4E43368F1AD7528F` (break `/Game/SuckItObjects/Structures/Struct_suckItItem` (`self.BaseInfo`))))
    (`TextRenderComponent.K2_SetText` (`/Game/SuckItObjects/BP_Tank.CurrentWeightDisplay` (`self.TankReference`)) (`KismetTextLibrary.Conv_DoubleToText` _tankinfo_weight "HalfToEven"))
    (`self.K2_DestroyActor`)
    (`/Game/SuckItObjects/BP_Tank.setTankScale` (`self.TankReference`) _returnvalue)
    (set `SpringArmComponent.TargetArmLength` (+ _returnvalue 100.0) (`/Game/SuckItObjects/BP_Tank.SpringArm` (`self.TankReference`)))))

(fn `UserConstructionScript`
  (bind _returnvalue (`KismetStringLibrary.Conv_StringToName` (`|GetEnumeratorNameAsString` (`self.itemMeshSelection`))))
  (bind _returnvalue_2 (`|GetDataTableRow` "/Game/SuckItObjects/Data_Tables/DT_SuckItItems.DT_SuckItItems" _returnvalue)
    (:`then`
      (`StaticMeshComponent.SetStaticMesh` (`self.Item`) (`.Mesh_12_8E714C364DD81D518DA64684CA241D6F` (break `/Game/SuckItObjects/Structures/Struct_suckItItem` _returnvalue_2)))
      (bind _returnvalue_3 (`|GetDataTableRow` "/Game/SuckItObjects/Data_Tables/DT_SuckItItems.DT_SuckItItems" _returnvalue)
        (:`then`
          (set `self.BaseInfo` _returnvalue_3))))
    (:`RowNotFound`
      (`KismetSystemLibrary.PrintString` "ITEM SELECTED NOT FOUND" false))))