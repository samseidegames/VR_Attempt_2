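; Player-possessable tank pawn with dual-track controls, a weight display set on BeginPlay and a starting scale set at construction.
; Left and right Enhanced Input axes store track speeds in the TankInfo struct and share one movement chain.
; Their difference yaws the tank, while a total scaled by actor size drives forward movement input.
; The logic that excludes floor meshes from object fading is disconnected.
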(event `self.ReceiveBeginPlay`
  (bind (_tankinfo_rotation _tankinfo_speed_r _tankinfo_speed_l _tankinfo_speed_total _tankinfo_scale _tankinfo_weight) (break `/Game/SuckItObjects/Structures/Struct_Tank` (`self.TankInfo`)))
  ;[1 1 1] BeginPlay
  (`TextRenderComponent.K2_SetText` (`self.CurrentWeightDisplay`) (`KismetTextLibrary.Conv_DoubleToText` _tankinfo_weight "HalfToEven")))

(event `EnhancedInput|/Game/VRTemplate/Input/Actions/IA_Tank_Controls_R`
  (params (ActionValue :type "Float (double-precision)") (ElapsedSeconds :type "Float (double-precision)") (TriggeredSeconds :type "Float (double-precision)") (InputAction :type "InputAction Object Reference" :default "/Game/VRTemplate/Input/Actions/IA_Tank_Controls_R.IA_Tank_Controls_R"))
  (bind _returnvalue_x (`KismetMathLibrary.BreakVector` (`self.GetActorScale3D`)))
  (bind _returnvalue (`self.GetActorForwardVector`))
  (bind _tankinfo (`self.TankInfo`))
  (bind _tankinfo_2 (`self.TankInfo`))
  (bind (_rotation _speed_r _speed_l) (break `/Game/SuckItObjects/Structures/Struct_Tank` _tankinfo))
  ;[1 1 1 1 17] Tank Controls v2
  (:`Triggered`
    (setmembers `/Game/SuckItObjects/Structures/Struct_Tank` :`StructRef` (`self.TankInfo`) :`Speed_R` ActionValue)
    (bind _structout (setmembers `/Game/SuckItObjects/Structures/Struct_Tank` :`StructRef` _tankinfo :`Speed_Total` (* (+ ActionValue (stale `EnhancedInput|/Game/VRTemplate/Input/Actions/IA_Tank_Controls_L` ActionValue)) _returnvalue_x) :!label _label))
    ;;[0.06771 0.06771 0.06771] Tank Rotate
    (if (>= _speed_r _speed_l)
      (setmembers `/Game/SuckItObjects/Structures/Struct_Tank` :`StructRef` _tankinfo_2 :`Rotation` (- _speed_l _speed_r))
      (else
        (bind (_rotation_2 _speed_r_2 _speed_l_2 _speed_total) (break `/Game/SuckItObjects/Structures/Struct_Tank` _structout))
        (setmembers `/Game/SuckItObjects/Structures/Struct_Tank` :`StructRef` _tankinfo_2 :`Rotation` (* (- _speed_r_2 _speed_l_2) -1.0))))
    (`self.K2_AddActorLocalRotation` (`KismetMathLibrary.MakeRotator` 0.0 0.0 (`.Rotation_2_ED1EBF5E47E523224D371FB4DC487099` (break `/Game/SuckItObjects/Structures/Struct_Tank` (`self.TankInfo`)))))
    ;;[0.07292 0.07292 0.07292] Tank forward and back
    (`self.AddMovementInput` (`KismetMathLibrary.Normal` _returnvalue) _speed_total)
    (`KismetSystemLibrary.PrintString` (`KismetStringLibrary.Conv_VectorToString` _returnvalue))))

(event `EnhancedInput|/Game/VRTemplate/Input/Actions/IA_Tank_Controls_L`
  (params (ActionValue :type "Float (double-precision)") (ElapsedSeconds :type "Float (double-precision)") (TriggeredSeconds :type "Float (double-precision)") (InputAction :type "InputAction Object Reference" :default "/Game/VRTemplate/Input/Actions/IA_Tank_Controls_L.IA_Tank_Controls_L"))
  ;[1 1 1 1 17] Tank Controls v2
  (:`Triggered`
    (setmembers `/Game/SuckItObjects/Structures/Struct_Tank` :`StructRef` (`self.TankInfo`) :`Speed_L` ActionValue)
    (goto _label)))

(event `PossessTank`
  ;[1 1 1] PossessTank
  (`Controller.Possess` (`GameplayStatics.GetPlayerController` 0) self))

(fn `setTankScale`
  (`self.SetActorScale3D` (0.2 0.2 0.2)))

(fn `UserConstructionScript`
  (bind _beginningtanksize (`/Game/SuckItObjects/General_BPs/TankSizeGlobals.Get Beginning Tank Size`))
  (`SceneComponent.SetWorldScale3D` (`self.RootComponent`) (`KismetMathLibrary.Conv_DoubleToVector` _beginningtanksize)))