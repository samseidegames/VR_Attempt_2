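; Medium suckable item (oven or table) that the VR pawn's tank absorbs, with mesh and mass set in the Construction Script.
; Once tank weight reaches the large-size threshold and the tank has entered the suck collision, Tick pulls the item toward it using delta-time-scaled local offsets.
; Touching the item collision destroys it, adds its mass to the pawn's total and rescales the tank if that exceeds the threshold.
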(event `self.ReceiveBeginPlay`
  ;[0.03434 0.03434 0.03434] Gets our Tank Instance
  (bind _outactors (`GameplayStatics.GetAllActorsOfClass` "/Game/SuckItObjects/BP_Tank.BP_Tank_C"))
  (for _array_element _outactors
    (if (`KismetSystemLibrary.IsValid` _array_element)
      (set `self.TankReference` _array_element)
      (bind _outactors_2 (`GameplayStatics.GetAllActorsOfClass` "/Game/VRTemplate/Blueprints/VRPawn.VRPawn_C"))
      (for _array_element_2 _outactors_2
        (set `self.VRPawnReference` _array_element_2)))))

(event `self.ReceiveTick`
  (params (DeltaSeconds :type "Float (single-precision)"))
  (bind _tanksizemax (`/Game/SuckItObjects/General_BPs/TankSizeGlobals.Get Large Tank Size`))
  (if (<= _tanksizemax (`/Game/VRTemplate/Blueprints/VRPawn.TankTotalWeight` (`self.VRPawnReference`)))
    (`self.Other Actor`
      (:`then`
        (`self.PullTowardsTank`))
      (:`else`))))

(event `self.SuckCollission.OnComponentBeginOverlap`
  (params (OverlappedComponent :type "PrimitiveComponent Object Reference") (OtherActor :type "Actor Object Reference") (OtherComp :type "PrimitiveComponent Object Reference") (OtherBodyIndex :type Integer) (bFromSweep :type Boolean) (SweepResult :type "HitResult Structure (by ref)"))
  (if (== OtherActor (`self.TankReference`))
    (set `self.Other Actor` OtherActor)))

(event `self.SuckCollission.OnComponentEndOverlap`
  (params (OverlappedComponent :type "PrimitiveComponent Object Reference") (OtherActor :type "Actor Object Reference") (OtherComp :type "PrimitiveComponent Object Reference") (OtherBodyIndex :type Integer)))

(event `PullTowardsTank`
  (`self.K2_AddActorLocalOffset` (* (`KismetMathLibrary.Normal` (- (`self.K2_GetActorLocation` (`self.TankReference`)) (`self.K2_GetActorLocation`))) (`GameplayStatics.GetWorldDeltaSeconds`) (`self.Speed`))))

(event `self.ItemCollission.OnComponentBeginOverlap`
  (params (OverlappedComponent :type "PrimitiveComponent Object Reference") (OtherActor :type "Actor Object Reference") (OtherComp :type "PrimitiveComponent Object Reference") (OtherBodyIndex :type Integer) (bFromSweep :type Boolean) (SweepResult :type "HitResult Structure (by ref)"))
  (bind _itemcollission (`self.ItemCollission`))
  (bind _suckcollission (`self.SuckCollission`))
  (bind _vrpawnreference (`self.VRPawnReference`))
  (if (== OtherActor (`self.TankReference`))
    (`PrimitiveComponent.SetCollisionEnabled` (`self.Item`) "NoCollision")
    (`/Engine/EditorBlueprintResources/StandardMacros.IsValid` _itemcollission
      (:`Is Valid`
        (`PrimitiveComponent.SetCollisionEnabled` _itemcollission "NoCollision"))
      (:`Is Not Valid`
        _))
    (`/Engine/EditorBlueprintResources/StandardMacros.IsValid` _suckcollission
      (:`Is Valid`
        (`PrimitiveComponent.SetCollisionEnabled` _suckcollission "NoCollision"))
      (:`Is Not Valid`
        _))
    (`self.K2_DestroyActor`)
    (`/Game/VRTemplate/Blueprints/VRPawn.UpdateTotalWeight` _vrpawnreference (`self.ItemMass`))
    (bind _tanksizemax (`/Game/SuckItObjects/General_BPs/TankSizeGlobals.Get Large Tank Size`))
    (if (> (`/Game/VRTemplate/Blueprints/VRPawn.TankTotalWeight` _vrpawnreference) _tanksizemax)
      (`SceneComponent.SetWorldScale3D` (`/Game/SuckItObjects/BP_Tank.Tank` (`self.TankReference`)) (0.4 0.4 0.4)))))

(fn `UserConstructionScript`
  (bind _item (`self.Item`))
  (switch `/Game/SuckItObjects/Medium_Items/BPs/MItemMeshOptions` (`self.ItemMesh`)
    (:`NewEnumerator3`
      (`StaticMeshComponent.SetStaticMesh` _item "/Game/SuckItObjects/Medium_Items/Oven.Oven")
      (set `self.ItemMesh` "NewEnumerator3")
      (set `self.ItemMass` 136.0))
    (:`NewEnumerator4`
      (`StaticMeshComponent.SetStaticMesh` _item "/Game/SuckItObjects/Medium_Items/Table.Table")
      (set `self.ItemMesh` "NewEnumerator4")
      (set `self.ItemMass` 60.0))))